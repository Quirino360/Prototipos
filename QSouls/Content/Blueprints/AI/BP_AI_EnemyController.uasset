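; Enemy AI controller that runs the BT_Enemy behavior tree and seeds its initial state.
; On BeginPlay it stores the player's third-person character as CurrentTarget and writes AIState to the blackboard.
; The perception update event is empty; the sight-based logic that sets or clears the TargetActor blackboard key is disconnected and never runs.
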(event OnTargetPerceptionUpdated(AIPerception)
  (params (Actor :type Actor%20Object%20Reference) (Stimulus :type AI%20Stimulus%20Structure)))

(event EventBeginPlay
  (AI|RunBehaviorTree "/Game/Blueprints/AI/BT_Enemy.BT_Enemy")
  (bind _asbp_3rd_person_character (Utilities|Casting|CastToBP_3rdPersonCharacter (Game|GetPlayerCharacter 0)))
  (Variables|Components|SetCurrentTarget _asbp_3rd_person_character)
  (AI|Components|Blackboard|SetValueasEnum (AI|GetBlackboard 0) (Utilities|Name|MakeLiteralName "AIState") (Variables|Components|GetAI_State)))

(event EventTick
  (params (DeltaSeconds :type Float%20%28single-precision%29)))

(fn ConstructionScript)